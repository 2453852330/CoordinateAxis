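; BP_AxisChecker picks axis handles under the mouse cursor and drives dragging of the actor that owns them, in the manner of a transform gizmo.
; While the left button is up, Tick traces from the cursor on one object type and uses the hit component's first tag to activate an axis, plane or XYZ handle through interface messages.
; While held, it sends move messages to that actor, and look input is ignored if a handle was hit.
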(event `Key|LeftMouseButton`
  (params (Key :type "Key Structure"))
  (:`Pressed`
    (set `self.bIsLeftMouseButtonDown` true)
    (bind _pc (`self.PC`)
      (:`then`
        (`Controller.SetIgnoreLookInput` _pc (`self.bIsHit`)))
      (:`else`)))
  (:`Released`
    (set `self.bIsLeftMouseButtonDown` false)
    (bind _pc_2 (`self.PC`)
      (:`then`
        (`Controller.SetIgnoreLookInput` _pc_2 false))
      (:`else`))))

(event `self.ReceiveTick`
  (params (DeltaSeconds :type "Float (single-precision)"))
  (bind _hitactor (`self.HitActor`))
  (bind _hitactor_2 (`self.HitActor`))
  (bind _hitactor_3 (`self.HitActor`))
  (bind _hitactor_4 (`self.HitActor`))
  (bind _hitactor_5 (`self.HitActor`))
  (bind _hitactor_6 (`self.HitActor`))
  (bind _hitactor_7 (`self.HitActor`))
  (if (`self.bIsLeftMouseButtonDown`)
    (bind _hitactor_8 (`self.HitActor`)
      (:`then`
        (message `/CoordinateAxis/BPI_ActiveAxis.BPI_HandleMove` _hitactor_8))
      (:`else`))
    (else
      (bind _pc (`self.PC`)
        (:`then`
          (bind (_outhit _returnvalue) (`self.LineTraceForCoordinate` _pc))
          (set `self.bIsHit` _returnvalue)
          (if _returnvalue
            ;[0 1 0.2734] hit handle
            (`|ExecutionSequence`
              (:`then_0`
                (bind (_bblockinghit _binitialoverlap _time _distance _location _impactpoint _normal _impactnormal _physmat _hitactor_9 _hitcomponent) (`GameplayStatics.BreakHitResult` _outhit))
                (set `self.HitActor` _hitactor_9)
                (set `self.HitPos` _impactpoint)
                (bind _output (`|GetArrayItem` (`ActorComponent.ComponentTags` _hitcomponent)))
                (if (not (`self.ActorHasTag` _hitactor_9 _output))
                  (switch `name` _output
                    (:`X`
                      (message `/CoordinateAxis/BPI_ActiveAxis.BPI_SetHitPos` _hitactor (`self.HitPos`))
                      (message `/CoordinateAxis/BPI_ActiveAxis.BPI_ActiveX` _hitactor))
                    (:`Y`
                      (message `/CoordinateAxis/BPI_ActiveAxis.BPI_SetHitPos` _hitactor_3 (`self.HitPos`))
                      (message `/CoordinateAxis/BPI_ActiveAxis.BPI_ActiveY` _hitactor_3))
                    (:`Z`
                      (message `/CoordinateAxis/BPI_ActiveAxis.BPI_SetHitPos` _hitactor_4 (`self.HitPos`))
                      (message `/CoordinateAxis/BPI_ActiveAxis.BPI_ActiveZ` _hitactor_4))
                    (:`XY`
                      (message `/CoordinateAxis/BPI_ActiveAxis.BPI_SetHitPos` _hitactor_5 (`self.HitPos`))
                      (message `/CoordinateAxis/BPI_ActiveAxis.BPI_ActiveXY` _hitactor_5))
                    (:`XZ`
                      (message `/CoordinateAxis/BPI_ActiveAxis.BPI_SetHitPos` _hitactor_6 (`self.HitPos`))
                      (message `/CoordinateAxis/BPI_ActiveAxis.BPI_ActiveXZ` _hitactor_6))
                    (:`YZ`
                      (message `/CoordinateAxis/BPI_ActiveAxis.BPI_SetHitPos` _hitactor_7 (`self.HitPos`))
                      (message `/CoordinateAxis/BPI_ActiveAxis.BPI_ActiveYZ` _hitactor_7))
                    (:`XYZ`
                      (message `/CoordinateAxis/BPI_ActiveAxis.BPI_SetHitPos` _hitactor_2 (`self.HitPos`))
                      (message `/CoordinateAxis/BPI_ActiveAxis.BPI_ActiveXYZ` _hitactor_2))))))
            (else
              (bind _hitactor_10 (`self.HitActor`)
                (:`then`
                  (message `/CoordinateAxis/BPI_ActiveAxis.BPI_DeactiveAll` _hitactor_10)
                  (set `self.HitActor` null))
                (:`else`)))))
        (:`else`)))))

(fn `LineTraceForCoordinate`
  (params (PC :type "PlayerController Object Reference"))
  (returns (OutHit :type "HitResult Structure") (ReturnValue :type Boolean))
  (bind (_worldlocation _worlddirection) (`PlayerController.DeprojectMousePositionToWorld` PC))
  (bind (_outhit _returnvalue) (`KismetSystemLibrary.LineTraceSingleForObjects` _worldlocation (+ _worldlocation (* _worlddirection 100000000.0)) (`|MakeArray` "ObjectTypeQuery7" :!type "EObjectTypeQuery Enum") true))
  (return _outhit _returnvalue))

(fn `UserConstructionScript`)