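; Rotation gizmo actor that rotates itself and its bound actor around a selected X, Y or Z axis as the mouse moves.
; Interface events store the active axis in the actor tag and highlight that axis's material.
; On move, the mouse's 0–360 screen angle around the projected hit point, measured from screen right via dot products, offsets the cached rotation's matching component.
; It sends guide-line endpoints and the angle to the player controller.
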(event `/CoordinateAxis/BPI_ActiveAxis.BPI_SetHitPos`
  (params (HitPos :type "Vector Structure"))
  ;[0 1 0.8125] receive hit pos
  (set `self.HitPos` HitPos)
  (set `self.CacheRotation` (`self.K2_GetActorRotation`))
  (bind _output_get (set `self.ScreenStartPos` (- (`WidgetLayoutLibrary.ProjectWorldLocationToWidgetPosition` (`GameplayStatics.GetPlayerController` 0) (`self.HitPos`)) (50.0 0.0))))
  ;[0.07812 0 1] call draw interface
  (message `/CoordinateAxis/Debug/BPI_DrawInfo.BPI_SendStart1` (`GameplayStatics.GetPlayerController` 0) _output_get))

(event `/CoordinateAxis/BPI_ActiveAxis.BPI_ActiveX`
  ;[1 0 0.09375] x
  (`self.BP_ChangeActorTag` "X")
  (`PrimitiveComponent.SetMaterial` (`self.AxisX`) 0 "/CoordinateAxis/Materials/MI_Active.MI_Active")
  (`PrimitiveComponent.SetMaterial` (`self.AxisY`) 0 "/CoordinateAxis/Materials/MI_Y.MI_Y")
  (`PrimitiveComponent.SetMaterial` (`self.AxisZ`) 0 "/CoordinateAxis/Materials/MI_Z.MI_Z"))

(event `/CoordinateAxis/BPI_ActiveAxis.BPI_ActiveY`
  ;[0.125 1 0] y
  (`self.BP_ChangeActorTag` "Y")
  (`PrimitiveComponent.SetMaterial` (`self.AxisX`) 0 "/CoordinateAxis/Materials/MI_X.MI_X")
  (`PrimitiveComponent.SetMaterial` (`self.AxisY`) 0 "/CoordinateAxis/Materials/MI_Active.MI_Active")
  (`PrimitiveComponent.SetMaterial` (`self.AxisZ`) 0 "/CoordinateAxis/Materials/MI_Z.MI_Z"))

(event `/CoordinateAxis/BPI_ActiveAxis.BPI_ActiveZ`
  ;[0 1 0.9531] z
  (`self.BP_ChangeActorTag` "Z")
  (`PrimitiveComponent.SetMaterial` (`self.AxisX`) 0 "/CoordinateAxis/Materials/MI_X.MI_X")
  (`PrimitiveComponent.SetMaterial` (`self.AxisY`) 0 "/CoordinateAxis/Materials/MI_Y.MI_Y")
  (`PrimitiveComponent.SetMaterial` (`self.AxisZ`) 0 "/CoordinateAxis/Materials/MI_Active.MI_Active"))

(event `/CoordinateAxis/BPI_ActiveAxis.BPI_HandleMove`
  (bind _returnvalue (`GameplayStatics.GetPlayerController` 0))
  (bind _screenstartpos (`self.ScreenStartPos`))
  ;[0.3828 1 0] handle move
  (`|ExecutionSequence`
    (:`then_0`
      (message `/CoordinateAxis/Debug/BPI_DrawInfo.BPI_SendStart2` _returnvalue _screenstartpos)
      (message `/CoordinateAxis/Debug/BPI_DrawInfo.BPI_SendEnd2` _returnvalue (+ _screenstartpos (200.0 0.0))))
    (:`then_1`
      (bind _returnvalue_2 (`WidgetLayoutLibrary.GetMousePositionOnViewport`))
      (bind _output_get (set `self.ScreenEndPos` _returnvalue_2))
      (message `/CoordinateAxis/Debug/BPI_DrawInfo.BPI_SendEnd1` (`GameplayStatics.GetPlayerController` 0) _output_get))
    (:`then_2`
      (switch `name` (`|GetArrayItem` (`self.Tags`))
        (:`X`
          (bind _output_get_2 (set `self.TargetRotation` (`KismetMathLibrary.MakeRotator` (+ (`self.CalcAngle`) (.roll (`self.CacheRotation`))) (.pitch (`self.CacheRotation`)) (.yaw (`self.CacheRotation`)))))
          (`self.K2_SetActorRotation` _output_get_2))
        (:`Y`
          (bind _output_get_3 (set `self.TargetRotation` (`KismetMathLibrary.MakeRotator` (.roll (`self.CacheRotation`)) (+ (`self.CalcAngle`) (.pitch (`self.CacheRotation`))) (.yaw (`self.CacheRotation`)))))
          (`self.K2_SetActorRotation` _output_get_3))
        (:`Z`
          (bind _output_get_4 (set `self.TargetRotation` (`KismetMathLibrary.MakeRotator` (.roll (`self.CacheRotation`)) (.pitch (`self.CacheRotation`)) (+ (`self.CalcAngle`) (.yaw (`self.CacheRotation`))))))
          (`self.K2_SetActorRotation` _output_get_4))))
    (:`then_3`
      (bind _bindactor (`self.BindActor`)
        (:`then`
          (`self.K2_SetActorRotation` _bindactor (`self.TargetRotation`) false))
        (:`else`)))))

(event `/CoordinateAxis/BPI_ActiveAxis.BPI_DeactiveAll`
  ;[1 0.6094 0] deactive all
  (`self.BP_ChangeActorTag` "N")
  (`PrimitiveComponent.SetMaterial` (`self.AxisX`) 0 "/CoordinateAxis/Materials/MI_X.MI_X")
  (`PrimitiveComponent.SetMaterial` (`self.AxisY`) 0 "/CoordinateAxis/Materials/MI_Y.MI_Y")
  (`PrimitiveComponent.SetMaterial` (`self.AxisZ`) 0 "/CoordinateAxis/Materials/MI_Z.MI_Z"))

(fn `CalcAngle`
  (returns (OutAngle :type "Float (double-precision)"))
  (bind _returnvalue (`KismetMathLibrary.Normal2D` (- (`self.ScreenEndPos`) (`self.ScreenStartPos`))))
  (bind _returnvalue_2 (`KismetMathLibrary.DegAcos` (`KismetMathLibrary.DotProduct2D` _returnvalue (`KismetMathLibrary.MakeVector2D` 1.0))))
  (bind _returnvalue_3 (`KismetMathLibrary.SelectFloat` _returnvalue_2 (- 360.0 _returnvalue_2) (>= (`KismetMathLibrary.DotProduct2D` _returnvalue (`KismetMathLibrary.MakeVector2D` 0.0 1.0)) 0.0)))
  (message `/CoordinateAxis/Debug/BPI_DrawInfo.BPI_SendAngle` (`GameplayStatics.GetPlayerController` 0) _returnvalue_3)
  (return _returnvalue_3))

(fn `UserConstructionScript`)