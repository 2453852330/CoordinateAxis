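; BP_MoveAxis is a translation gizmo that moves itself and a bound StaticMeshActor tagged "A".
; Interface events highlight the active axis, plane or center, store it as the actor tag and cache start positions.
; Dragging scales mouse delta along that direction (planes use one fixed vector), signed against the screen-projected hit direction; center follows the cursor ray at cached distance.
; A debug widget shows drag points; F randomizes both actors' rotation.
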(event `/CoordinateAxis/BPI_ActiveAxis.BPI_ActiveXY`
  ;[0.9922 1 0] XY
  (`|ExecutionSequence`
    (:`then_0`
      (`PrimitiveComponent.SetMaterial` (`self.AxisX`) 0 "/CoordinateAxis/Materials/MI_Active.MI_Active")
      (`PrimitiveComponent.SetMaterial` (`self.AxisY`) 0 "/CoordinateAxis/Materials/MI_Active.MI_Active")
      (`PrimitiveComponent.SetMaterial` (`self.AxisZ`) 0 "/CoordinateAxis/Materials/MI_Z.MI_Z"))
    (:`then_1`
      (`PrimitiveComponent.SetMaterial` (`self.AxisXY`) 0 "/CoordinateAxis/Materials/MI_Active.MI_Active")
      (`PrimitiveComponent.SetMaterial` (`self.AxisYZ`) 0 "/CoordinateAxis/Materials/MI_Plane.MI_Plane")
      (`PrimitiveComponent.SetMaterial` (`self.AxisXZ`) 0 "/CoordinateAxis/Materials/MI_Plane.MI_Plane"))
    (:`then_2`
      (`PrimitiveComponent.SetMaterial` (`self.AxisXYZ`) 0 "/CoordinateAxis/Materials/MI_Center.MI_Center")
      (`self.BP_ChangeActorTag` "XY")
      (`self.HandleAllState`))))

(event `/CoordinateAxis/BPI_ActiveAxis.BPI_ActiveXYZ`
  ;[0.6641 0 1] center
  (`|ExecutionSequence`
    (:`then_0`
      (`PrimitiveComponent.SetMaterial` (`self.AxisX`) 0 "/CoordinateAxis/Materials/MI_Active.MI_Active")
      (`PrimitiveComponent.SetMaterial` (`self.AxisY`) 0 "/CoordinateAxis/Materials/MI_Active.MI_Active")
      (`PrimitiveComponent.SetMaterial` (`self.AxisZ`) 0 "/CoordinateAxis/Materials/MI_Active.MI_Active"))
    (:`then_1`
      (`PrimitiveComponent.SetMaterial` (`self.AxisXY`) 0 "/CoordinateAxis/Materials/MI_Active.MI_Active")
      (`PrimitiveComponent.SetMaterial` (`self.AxisYZ`) 0 "/CoordinateAxis/Materials/MI_Active.MI_Active")
      (`PrimitiveComponent.SetMaterial` (`self.AxisXZ`) 0 "/CoordinateAxis/Materials/MI_Active.MI_Active"))
    (:`then_2`
      (`PrimitiveComponent.SetMaterial` (`self.AxisXYZ`) 0 "/CoordinateAxis/Materials/MI_Center.MI_Center")
      (`self.BP_ChangeActorTag` "XYZ")
      (`self.HandleAllState`))))

(event `/CoordinateAxis/BPI_ActiveAxis.BPI_ActiveX`
  ;[0 0.8359 1] X
  (`|ExecutionSequence`
    (:`then_0`
      (`PrimitiveComponent.SetMaterial` (`self.AxisX`) 0 "/CoordinateAxis/Materials/MI_Active.MI_Active")
      (`PrimitiveComponent.SetMaterial` (`self.AxisY`) 0 "/CoordinateAxis/Materials/MI_Y.MI_Y")
      (`PrimitiveComponent.SetMaterial` (`self.AxisZ`) 0 "/CoordinateAxis/Materials/MI_Z.MI_Z"))
    (:`then_1`
      (`PrimitiveComponent.SetMaterial` (`self.AxisXY`) 0 "/CoordinateAxis/Materials/MI_Plane.MI_Plane")
      (`PrimitiveComponent.SetMaterial` (`self.AxisYZ`) 0 "/CoordinateAxis/Materials/MI_Plane.MI_Plane")
      (`PrimitiveComponent.SetMaterial` (`self.AxisXZ`) 0 "/CoordinateAxis/Materials/MI_Plane.MI_Plane"))
    (:`then_2`
      (`PrimitiveComponent.SetMaterial` (`self.AxisXYZ`) 0 "/CoordinateAxis/Materials/MI_Center.MI_Center"))
    (:`then_3`
      (`self.BP_ChangeActorTag` "X")
      (`self.HandleAllState`))))

(event `/CoordinateAxis/BPI_ActiveAxis.BPI_ActiveXZ`
  ;[0 0.6016 1] XZ
  (`|ExecutionSequence`
    (:`then_0`
      (`PrimitiveComponent.SetMaterial` (`self.AxisX`) 0 "/CoordinateAxis/Materials/MI_Active.MI_Active")
      (`PrimitiveComponent.SetMaterial` (`self.AxisY`) 0 "/CoordinateAxis/Materials/MI_Y.MI_Y")
      (`PrimitiveComponent.SetMaterial` (`self.AxisZ`) 0 "/CoordinateAxis/Materials/MI_Active.MI_Active"))
    (:`then_1`
      (`PrimitiveComponent.SetMaterial` (`self.AxisXY`) 0 "/CoordinateAxis/Materials/MI_Plane.MI_Plane")
      (`PrimitiveComponent.SetMaterial` (`self.AxisYZ`) 0 "/CoordinateAxis/Materials/MI_Plane.MI_Plane")
      (`PrimitiveComponent.SetMaterial` (`self.AxisXZ`) 0 "/CoordinateAxis/Materials/MI_Active.MI_Active"))
    (:`then_2`
      (`PrimitiveComponent.SetMaterial` (`self.AxisXYZ`) 0 "/CoordinateAxis/Materials/MI_Center.MI_Center")
      (`self.BP_ChangeActorTag` "XZ")
      (`self.HandleAllState`))))

(event `/CoordinateAxis/BPI_ActiveAxis.BPI_DeactiveAll`
  ;[0.7578 0 1] Deactive All
  (`|ExecutionSequence`
    (:`then_0`
      (`PrimitiveComponent.SetMaterial` (`self.AxisX`) 0 "/CoordinateAxis/Materials/MI_X.MI_X")
      (`PrimitiveComponent.SetMaterial` (`self.AxisY`) 0 "/CoordinateAxis/Materials/MI_Y.MI_Y")
      (`PrimitiveComponent.SetMaterial` (`self.AxisZ`) 0 "/CoordinateAxis/Materials/MI_Z.MI_Z"))
    (:`then_1`
      (`PrimitiveComponent.SetMaterial` (`self.AxisXY`) 0 "/CoordinateAxis/Materials/MI_Plane.MI_Plane")
      (`PrimitiveComponent.SetMaterial` (`self.AxisYZ`) 0 "/CoordinateAxis/Materials/MI_Plane.MI_Plane")
      (`PrimitiveComponent.SetMaterial` (`self.AxisXZ`) 0 "/CoordinateAxis/Materials/MI_Plane.MI_Plane"))
    (:`then_2`
      (`PrimitiveComponent.SetMaterial` (`self.AxisXYZ`) 0 "/CoordinateAxis/Materials/MI_Center.MI_Center")
      (`self.BP_ChangeActorTag` "NULL")
      (`self.HandleAllState`))))

(event `/CoordinateAxis/BPI_ActiveAxis.BPI_ActiveY`
  ;[1 0.2812 0] Y
  (`|ExecutionSequence`
    (:`then_0`
      (`PrimitiveComponent.SetMaterial` (`self.AxisX`) 0 "/CoordinateAxis/Materials/MI_X.MI_X")
      (`PrimitiveComponent.SetMaterial` (`self.AxisY`) 0 "/CoordinateAxis/Materials/MI_Active.MI_Active")
      (`PrimitiveComponent.SetMaterial` (`self.AxisZ`) 0 "/CoordinateAxis/Materials/MI_Z.MI_Z"))
    (:`then_1`
      (`PrimitiveComponent.SetMaterial` (`self.AxisXY`) 0 "/CoordinateAxis/Materials/MI_Plane.MI_Plane")
      (`PrimitiveComponent.SetMaterial` (`self.AxisYZ`) 0 "/CoordinateAxis/Materials/MI_Plane.MI_Plane")
      (`PrimitiveComponent.SetMaterial` (`self.AxisXZ`) 0 "/CoordinateAxis/Materials/MI_Plane.MI_Plane"))
    (:`then_2`
      (`PrimitiveComponent.SetMaterial` (`self.AxisXYZ`) 0 "/CoordinateAxis/Materials/MI_Center.MI_Center"))
    (:`then_3`
      (`self.BP_ChangeActorTag` "Y")
      (`self.HandleAllState`))))

(event `/CoordinateAxis/BPI_ActiveAxis.BPI_ActiveYZ`
  ;[0 0.3672 1] YZ
  (`|ExecutionSequence`
    (:`then_0`
      (`PrimitiveComponent.SetMaterial` (`self.AxisX`) 0 "/CoordinateAxis/Materials/MI_X.MI_X")
      (`PrimitiveComponent.SetMaterial` (`self.AxisY`) 0 "/CoordinateAxis/Materials/MI_Active.MI_Active")
      (`PrimitiveComponent.SetMaterial` (`self.AxisZ`) 0 "/CoordinateAxis/Materials/MI_Active.MI_Active"))
    (:`then_1`
      (`PrimitiveComponent.SetMaterial` (`self.AxisXY`) 0 "/CoordinateAxis/Materials/MI_Plane.MI_Plane")
      (`PrimitiveComponent.SetMaterial` (`self.AxisYZ`) 0 "/CoordinateAxis/Materials/MI_Active.MI_Active")
      (`PrimitiveComponent.SetMaterial` (`self.AxisXZ`) 0 "/CoordinateAxis/Materials/MI_Plane.MI_Plane"))
    (:`then_2`
      (`PrimitiveComponent.SetMaterial` (`self.AxisXYZ`) 0 "/CoordinateAxis/Materials/MI_Center.MI_Center")
      (`self.BP_ChangeActorTag` "YZ")
      (`self.HandleAllState`))))

(event `/CoordinateAxis/BPI_ActiveAxis.BPI_ActiveZ`
  ;[1 0 0.7734] Z
  (`|ExecutionSequence`
    (:`then_0`
      (`PrimitiveComponent.SetMaterial` (`self.AxisX`) 0 "/CoordinateAxis/Materials/MI_X.MI_X")
      (`PrimitiveComponent.SetMaterial` (`self.AxisY`) 0 "/CoordinateAxis/Materials/MI_Y.MI_Y")
      (`PrimitiveComponent.SetMaterial` (`self.AxisZ`) 0 "/CoordinateAxis/Materials/MI_Active.MI_Active"))
    (:`then_1`
      (`PrimitiveComponent.SetMaterial` (`self.AxisXY`) 0 "/CoordinateAxis/Materials/MI_Plane.MI_Plane")
      (`PrimitiveComponent.SetMaterial` (`self.AxisYZ`) 0 "/CoordinateAxis/Materials/MI_Plane.MI_Plane")
      (`PrimitiveComponent.SetMaterial` (`self.AxisXZ`) 0 "/CoordinateAxis/Materials/MI_Plane.MI_Plane"))
    (:`then_2`
      (`PrimitiveComponent.SetMaterial` (`self.AxisXYZ`) 0 "/CoordinateAxis/Materials/MI_Center.MI_Center"))
    (:`then_3`
      (`self.BP_ChangeActorTag` "Z")
      (`self.HandleAllState`))))

(event `self.ReceiveBeginPlay`
  (bind _returnvalue (`GameplayStatics.GetPlayerController` 0))
  ;[0.8047 0 1] begin
  (`self.EnableInput` _returnvalue)
  (bind _returnvalue_2 (`|CreateWidget` "/CoordinateAxis/Debug/UI_DebugView.UI_DebugView_C" _returnvalue))
  (bind _output_get (set `self.UI_Debug` _returnvalue_2))
  (`UserWidget.AddToViewport` _output_get 0)
  (bind _outactors (`GameplayStatics.GetAllActorsOfClassWithTag` "/Script/Engine.StaticMeshActor" "A"))
  ;[0.125 1 0] set bind actor
  (set `self.BindActor` (`|GetArrayItem` _outactors)))

(event `Key|F`
  (params (Key :type "Key Structure"))
  (:`Pressed`
    (bind _bindactor (`self.BindActor`)
      (:`then`
        (bind _output_get (set `self.TmpRotator` (`KismetMathLibrary.MakeRotator` (`KismetMathLibrary.RandomFloatInRange` 0.0 360.0) (`KismetMathLibrary.RandomFloatInRange` 0.0 360.0) (`KismetMathLibrary.RandomFloatInRange` 0.0 360.0))))
        (`self.K2_SetActorRotation` _bindactor _output_get false)
        (`self.K2_SetActorRotation` _output_get))
      (:`else`))))

(event `/CoordinateAxis/BPI_ActiveAxis.BPI_SetHitPos`
  (params (HitPos :type "Vector Structure"))
  ;[0.6172 0 1] receive hit pos
  (set `self.HitPos` HitPos))

(event `/CoordinateAxis/BPI_ActiveAxis.BPI_HandleMove`
  ;[0.4297 1 0] Handle Move
  (`|ExecutionSequence`
    (:`then_0`
      (bind _returnvalue (`WidgetLayoutLibrary.GetMousePositionOnViewport`))
      (set `self.MouseOffset` (- _returnvalue (`self.StartPos`)))
      (bind _ui_debug (`self.UI_Debug`)
        (:`then`
          (set `/CoordinateAxis/Debug/UI_DebugView.PointEnd` _returnvalue _ui_debug))
        (:`else`)))
    (:`then_1`
      (bind (_offset _bisxyz) (`self.CalcPosOffset` 1.0))
      (if _bisxyz
        (bind _returnvalue_2 (+ _offset (`self.K2_GetActorLocation` (`GameplayStatics.GetPlayerPawn` 0))))
        (`self.K2_SetActorLocation` _returnvalue_2)
        (bind _bindactor (`self.BindActor`)
          (:`then`
            (`self.K2_SetActorLocation` _bindactor _returnvalue_2 false false))
          (:`else`))
        (else
          (bind _returnvalue_3 (+ (`self.CacheActorPos`) _offset))
          (`self.K2_SetActorLocation` _returnvalue_3)
          (bind _bindactor_2 (`self.BindActor`)
            (:`then`
              (`self.K2_SetActorLocation` _bindactor_2 _returnvalue_3 false false))
            (:`else`)))))))

(fn `CalcPosOffset`
  (params (Multi :type "Float (double-precision)" :default 1.0))
  (returns (Offset :type "Vector Structure") (bIsXYZ :type Boolean))
  (bind _mouseoffset (`self.MouseOffset`))
  (bind _mouseoffset_2 (`self.MouseOffset`))
  (bind _mouseoffset_3 (`self.MouseOffset`))
  (bind _mouseoffset_4 (`self.MouseOffset`))
  (bind _mouseoffset_5 (`self.MouseOffset`))
  (bind _mouseoffset_6 (`self.MouseOffset`))
  (switch `name` (`|GetArrayItem` (`self.Tags`))
    (:`X`
      ;[1 0.4453 0] X
      (return (* (`SceneComponent.GetUpVector` (`self.AxisX`)) (* (`KismetMathLibrary.SelectFloat` 1.0 -1.0 (>= (`KismetMathLibrary.DotProduct2D` (`self.WorldMoveDirToScreen`) (`KismetMathLibrary.Normal2D` _mouseoffset)) 0.0)) (`KismetMathLibrary.Abs` (`KismetMathLibrary.BreakVector2D` _mouseoffset)) (`local.Multi`))) false))
    (:`Y`
      ;[1 0.3984 0] Y
      (return (* (`SceneComponent.GetUpVector` (`self.AxisY`)) (* (`KismetMathLibrary.SelectFloat` 1.0 -1.0 (>= (`KismetMathLibrary.DotProduct2D` (`self.WorldMoveDirToScreen`) (`KismetMathLibrary.Normal2D` _mouseoffset_2)) 0.0)) (`KismetMathLibrary.Abs` (`KismetMathLibrary.BreakVector2D` _mouseoffset_2)) (`local.Multi`))) false))
    (:`Z`
      ;[0.5703 1 0] Z
      (return (* (`SceneComponent.GetUpVector` (`self.AxisZ`)) (* (`KismetMathLibrary.SelectFloat` 1.0 -1.0 (>= (`KismetMathLibrary.DotProduct2D` (`self.WorldMoveDirToScreen`) (`KismetMathLibrary.Normal2D` _mouseoffset_3)) 0.0)) (`KismetMathLibrary.Abs` (`.Y` (`KismetMathLibrary.BreakVector2D` _mouseoffset_3))) (`local.Multi`))) false))
    (:`XY`
      ;[0.6172 1 0] xz
      (return (* (`KismetMathLibrary.Normal` (- (`SceneComponent.K2_GetComponentLocation` (`self.xy`)) (`SceneComponent.K2_GetComponentLocation` (`self.AxisXY`)))) (* (`KismetMathLibrary.SelectFloat` 1.0 -1.0 (>= (`KismetMathLibrary.DotProduct2D` (`self.WorldMoveDirToScreen`) (`KismetMathLibrary.Normal2D` _mouseoffset_4)) 0.0)) (`KismetMathLibrary.Abs` (`KismetMathLibrary.BreakVector2D` _mouseoffset_4)) (`local.Multi`))) false))
    (:`XZ`
      ;[0.6172 1 0] xz
      (return (* (`KismetMathLibrary.Normal` (- (`SceneComponent.K2_GetComponentLocation` (`self.xz`)) (`SceneComponent.K2_GetComponentLocation` (`self.AxisXZ`)))) (* (`KismetMathLibrary.SelectFloat` 1.0 -1.0 (>= (`KismetMathLibrary.DotProduct2D` (`self.WorldMoveDirToScreen`) (`KismetMathLibrary.Normal2D` _mouseoffset_5)) 0.0)) (`KismetMathLibrary.Abs` (`KismetMathLibrary.BreakVector2D` _mouseoffset_5)) (`local.Multi`))) false))
    (:`YZ`
      ;[0.6172 1 0] yz
      (return (* (`KismetMathLibrary.Normal` (- (`SceneComponent.K2_GetComponentLocation` (`self.yz`)) (`SceneComponent.K2_GetComponentLocation` (`self.AxisYZ`)))) (* (`KismetMathLibrary.SelectFloat` 1.0 -1.0 (>= (`KismetMathLibrary.DotProduct2D` (`self.WorldMoveDirToScreen`) (`KismetMathLibrary.Normal2D` _mouseoffset_6)) 0.0)) (`KismetMathLibrary.Abs` (`KismetMathLibrary.BreakVector2D` _mouseoffset_6)) (`local.Multi`))) false))
    (:`XYZ`
      ;[0.6172 1 0] xyz
      (return (* (`.WorldDirection` (`PlayerController.DeprojectMousePositionToWorld` (`GameplayStatics.GetPlayerController` 0))) (`KismetMathLibrary.Vector_Distance` (`self.CacheActorPos`) (`self.K2_GetActorLocation` (`GameplayStatics.GetPlayerPawn` 0)))) true))))

(fn `HandleAllState`
  (locals (move_start :type "Vector2D Structure") (move_end :type "Vector2D Structure"))
  (bind _returnvalue (`self.K2_GetActorLocation`))
  (bind _returnvalue_2 (`GameplayStatics.GetPlayerController` 0))
  (`|ExecutionSequence`
    (:`then_0`
      (set `self.CacheActorPos` _returnvalue)
      ;[0 1 0.5547] calc mouse start pos on screen
      (bind _returnvalue_3 (`WidgetLayoutLibrary.GetMousePositionOnViewport`))
      (set `self.StartPos` _returnvalue_3)
      (set `local.move_start` (`WidgetLayoutLibrary.ProjectWorldLocationToWidgetPosition` _returnvalue_2 _returnvalue))
      (set `local.move_end` (`WidgetLayoutLibrary.ProjectWorldLocationToWidgetPosition` _returnvalue_2 (`self.HitPos`)))
      (set `self.WorldMoveDirToScreen` (`KismetMathLibrary.Normal2D` (- (`local.move_end`) (`local.move_start`)))))
    (:`then_1`
      (bind _ui_debug (`self.UI_Debug`)
        (:`then`
          (set `/CoordinateAxis/Debug/UI_DebugView.PointStart` (`self.StartPos`) _ui_debug)
          (set `/CoordinateAxis/Debug/UI_DebugView.MoveStart` (`local.move_start`) _ui_debug)
          (set `/CoordinateAxis/Debug/UI_DebugView.MoveEnd` (`local.move_end`) _ui_debug))
        (:`else`)))))

(fn `UserConstructionScript`)