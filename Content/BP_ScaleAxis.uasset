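; BP_ScaleAxis is a scale gizmo that resizes a bound actor, the first StaticMeshActor tagged "R", along X, Y, Z or all axes.
; Interface events store the active axis in the actor's tag, swap highlight materials, and cache the hit's screen position and starting scale.
; On move, mouse offset is projected onto the axis's screen direction (horizontal for XYZ), weighted by horizontal travel over viewport width, and added to cached scale.
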(event `/CoordinateAxis/BPI_ActiveAxis.BPI_SetHitPos`
  (params (HitPos :type "Vector Structure"))
  ;[1 0.09375 0] receive hit pos
  (bind _output_get (set `self.HitPos` HitPos))
  (set `self.ScreenStartPos` (`WidgetLayoutLibrary.ProjectWorldLocationToWidgetPosition` (`GameplayStatics.GetPlayerController` 0) _output_get))
  (bind _bindactor (`self.BindActor`)
    (:`then`
      (set `self.CacheScale` (`self.GetActorScale3D` _bindactor)))
    (:`else`)))

(event `/CoordinateAxis/BPI_ActiveAxis.BPI_ActiveX`
  ;[0.5469 1 0] x
  (`self.BP_ChangeActorTag` "X")
  (`PrimitiveComponent.SetMaterial` (`self.AxisX`) 0 "/CoordinateAxis/Materials/MI_Active.MI_Active")
  (`PrimitiveComponent.SetMaterial` (`self.AxisY`) 0 "/CoordinateAxis/Materials/MI_Y.MI_Y")
  (`PrimitiveComponent.SetMaterial` (`self.AxisZ`) 0 "/CoordinateAxis/Materials/MI_Z.MI_Z")
  (`PrimitiveComponent.SetMaterial` (`self.Center`) 0 "/CoordinateAxis/Materials/MI_Center.MI_Center"))

(event `/CoordinateAxis/BPI_ActiveAxis.BPI_ActiveY`
  ;[1 0 0.4219] y
  (`self.BP_ChangeActorTag` "Y")
  (`PrimitiveComponent.SetMaterial` (`self.AxisX`) 0 "/CoordinateAxis/Materials/MI_X.MI_X")
  (`PrimitiveComponent.SetMaterial` (`self.AxisY`) 0 "/CoordinateAxis/Materials/MI_Active.MI_Active")
  (`PrimitiveComponent.SetMaterial` (`self.AxisZ`) 0 "/CoordinateAxis/Materials/MI_Z.MI_Z")
  (`PrimitiveComponent.SetMaterial` (`self.Center`) 0 "/CoordinateAxis/Materials/MI_Center.MI_Center"))

(event `/CoordinateAxis/BPI_ActiveAxis.BPI_ActiveZ`
  ;[1 0 0.5625] z
  (`self.BP_ChangeActorTag` "Z")
  (`PrimitiveComponent.SetMaterial` (`self.AxisX`) 0 "/CoordinateAxis/Materials/MI_X.MI_X")
  (`PrimitiveComponent.SetMaterial` (`self.AxisY`) 0 "/CoordinateAxis/Materials/MI_Y.MI_Y")
  (`PrimitiveComponent.SetMaterial` (`self.AxisZ`) 0 "/CoordinateAxis/Materials/MI_Active.MI_Active")
  (`PrimitiveComponent.SetMaterial` (`self.Center`) 0 "/CoordinateAxis/Materials/MI_Center.MI_Center"))

(event `/CoordinateAxis/BPI_ActiveAxis.BPI_ActiveXYZ`
  ;[1 0.07031 0] xyz
  (`self.BP_ChangeActorTag` "XYZ")
  (`PrimitiveComponent.SetMaterial` (`self.AxisX`) 0 "/CoordinateAxis/Materials/MI_Active.MI_Active")
  (`PrimitiveComponent.SetMaterial` (`self.AxisY`) 0 "/CoordinateAxis/Materials/MI_Active.MI_Active")
  (`PrimitiveComponent.SetMaterial` (`self.AxisZ`) 0 "/CoordinateAxis/Materials/MI_Active.MI_Active")
  (`PrimitiveComponent.SetMaterial` (`self.Center`) 0 "/CoordinateAxis/Materials/MI_Center.MI_Center"))

(event `/CoordinateAxis/BPI_ActiveAxis.BPI_DeactiveAll`
  ;[0.6875 0 1] deactive all
  (`self.BP_ChangeActorTag` "N")
  (`PrimitiveComponent.SetMaterial` (`self.AxisX`) 0 "/CoordinateAxis/Materials/MI_X.MI_X")
  (`PrimitiveComponent.SetMaterial` (`self.AxisY`) 0 "/CoordinateAxis/Materials/MI_Y.MI_Y")
  (`PrimitiveComponent.SetMaterial` (`self.AxisZ`) 0 "/CoordinateAxis/Materials/MI_Z.MI_Z")
  (`PrimitiveComponent.SetMaterial` (`self.Center`) 0 "/CoordinateAxis/Materials/MI_Center.MI_Center"))

(event `/CoordinateAxis/BPI_ActiveAxis.BPI_HandleMove`
  (bind _calcedscaleoffset (`self.CalcedScaleOffset`))
  ;[0.3125 1 0] handle move
  (`|ExecutionSequence`
    (:`then_0`
      (`self.CalcWorldDirToScreen`)
      (bind _result (`self.CalcScaleIntensity`))
      (set `self.CalcedScaleOffset` _result)
      (switch `name` (`|GetArrayItem` (`self.Tags`))
        (:`X`
          (set `self.TargetScale` (+ (`self.CacheScale`) (`KismetMathLibrary.MakeVector` (`self.CalcedScaleOffset`)))))
        (:`Y`
          (set `self.TargetScale` (+ (`self.CacheScale`) (`KismetMathLibrary.MakeVector` 0.0 (`self.CalcedScaleOffset`)))))
        (:`Z`
          (set `self.TargetScale` (+ (`self.CacheScale`) (`KismetMathLibrary.MakeVector` 0.0 0.0 (`self.CalcedScaleOffset`)))))
        (:`XYZ`
          (set `self.TargetScale` (+ (`self.CacheScale`) (`KismetMathLibrary.MakeVector` _calcedscaleoffset _calcedscaleoffset _calcedscaleoffset))))))
    (:`then_1`
      (bind _bindactor (`self.BindActor`)
        (:`then`
          (`self.SetActorScale3D` _bindactor (`self.TargetScale`)))
        (:`else`)))))

(event `self.ReceiveBeginPlay`
  ;[0.5469 1 0] begin
  (`|ExecutionSequence`
    (:`then_0`
      (bind _outactors (`GameplayStatics.GetAllActorsOfClassWithTag` "/Script/Engine.StaticMeshActor" "R"))
      (set `self.BindActor` (`|GetArrayItem` _outactors)))
    (:`then_1`
      (bind _asbp_game_mode_debug_axis (cast `/CoordinateAxis/Debug/BP_GameMode_DebugAxis` (`GameplayStatics.GetGameMode`)))
      (set `self.CacheGameModeForDebug` _asbp_game_mode_debug_axis))))

(fn `CalcScaleIntensity`
  (returns (Result :type "Float (double-precision)"))
  (locals (Offset :type "Vector2D Structure") (Length :type "Float (double-precision)" :default 0.0))
  (`|ExecutionSequence`
    (:`then_0`
      (bind _returnvalue (`WidgetLayoutLibrary.GetMousePositionOnViewport`))
      (set `local.Offset` (- _returnvalue (`self.ScreenStartPos`))))
    (:`then_1`
      (bind _output_get (set `local.Length` (`KismetMathLibrary.DotProduct2D` (`local.Offset`) (`self.WorldDirOnScreen`))))
      (set `local.Length` (* _output_get (/ (`KismetMathLibrary.Abs` (`KismetMathLibrary.BreakVector2D` (`local.Offset`))) (`KismetMathLibrary.BreakVector2D` (`WidgetLayoutLibrary.GetViewportSize`))))))
    (:`then_2`
      (if (== (`|GetArrayItem` (`self.Tags`)) "XYZ")
        (set `local.Length` (* (`KismetMathLibrary.DotProduct2D` (`local.Offset`) (1.0 0.0)) (/ (`KismetMathLibrary.Abs` (`KismetMathLibrary.BreakVector2D` (`local.Offset`))) (`KismetMathLibrary.BreakVector2D` (`WidgetLayoutLibrary.GetViewportSize`)))))))
    (:`then_4`
      (return (`local.Length`)))))

(fn `CalcWorldDirToScreen`
  (locals (start :type "Vector2D Structure") (Dir :type "Vector Structure" :default (0.0 0.0 0.0)) (End :type "Vector2D Structure"))
  (`|ExecutionSequence`
    (:`then_0`
      (set `local.start` (`WidgetLayoutLibrary.ProjectWorldLocationToWidgetPosition` (`GameplayStatics.GetPlayerController` 0) (`self.K2_GetActorLocation`)))
      (switch `name` (`|GetArrayItem` (`self.Tags`))
        (:`X`
          (set `local.Dir` (`SceneComponent.GetUpVector` (`self.AxisX`))))
        (:`Y`
          (set `local.Dir` (`SceneComponent.GetUpVector` (`self.AxisY`))))
        (:`Z`
          (set `local.Dir` (`SceneComponent.GetUpVector` (`self.AxisZ`))))))
    (:`then_1`
      (set `local.End` (`WidgetLayoutLibrary.ProjectWorldLocationToWidgetPosition` (`GameplayStatics.GetPlayerController` 0) (+ (`self.K2_GetActorLocation`) (* (`local.Dir`) 50.0)))))
    (:`then_2`
      (set `self.WorldDirOnScreen` (`KismetMathLibrary.Normal2D` (- (`local.End`) (`local.start`)))))))

(fn `UserConstructionScript`)