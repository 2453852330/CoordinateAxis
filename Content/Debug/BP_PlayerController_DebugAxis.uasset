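; Debug player controller for testing a coordinate-axis transform gizmo driven by the GISCoordinateAxisManager subsystem.
; On BeginPlay it adds debug-view and mode-manager widgets to the viewport.
; Left click, unless a handle is moving, line-traces under the cursor and sets an "AAA"-tagged actor as the work mesh, or clears it otherwise.
; Interface events feed move points and angle into the debug widget, whose points reset on mouse release.
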(event `self.ReceiveBeginPlay`
  ;[0 0.4375 1] begin
  (`|ExecutionSequence`
    (:`then_0`
      (bind _returnvalue (`|CreateWidget` "/CoordinateAxis/Debug/UI_DebugView.UI_DebugView_C" self))
      (bind _output_get (set `self.UI_Debug` _returnvalue))
      (`UserWidget.AddToViewport` _output_get 0))
    (:`then_1`
      (bind _returnvalue_2 (`|CreateWidget` "/CoordinateAxis/Debug/UI_ModeManager.UI_ModeManager_C" self))
      (bind _output_get_2 (set `self.UI_ModeManager` _returnvalue_2))
      (`UserWidget.AddToViewport` _output_get_2 0))))

(event `Key|LeftMouseButton`
  (params (Key :type "Key Structure"))
  (bind (_worldlocation _worlddirection) (`self.DeprojectMousePositionToWorld`))
  (:`Pressed`
    (if (not (`GISCoordinateAxisManager.bIsHandleMove` (subsystem `GISCoordinateAxisManager`)))
      (bind (_outhit _returnvalue) (`KismetSystemLibrary.LineTraceSingle` _worldlocation (+ _worldlocation (* _worlddirection 100000000.0)) "TraceTypeQuery1" true))
      (bind (_bblockinghit _binitialoverlap _time _distance _location _impactpoint _normal _impactnormal _physmat _hitactor) (`GameplayStatics.BreakHitResult` _outhit))
      (if (and (`KismetSystemLibrary.IsValid` _hitactor) _returnvalue)
        (if (`self.ActorHasTag` _hitactor "AAA")
          ;[0 0.8594 1] subsystem interface
          (`GISCoordinateAxisManager.BP_SetWorkMeshActor` (subsystem `GISCoordinateAxisManager`) _hitactor)
          (else
            (`GISCoordinateAxisManager.BP_SetWorkMeshActor` (subsystem `GISCoordinateAxisManager`) null :!label _label)))
        (else
          (goto _label)))))
  (:`Released`
    (bind _ui_debug (`self.UI_Debug`)
      (:`then`
        (`/CoordinateAxis/Debug/UI_DebugView.ResetAllPoint` _ui_debug))
      (:`else`))))

(event `/CoordinateAxis/Debug/BPI_DrawInfo.BPI_SendStart2`
  (params (Point :type "Vector2D Structure"))
  (bind _ui_debug (`self.UI_Debug`)
    (:`then`
      (set `/CoordinateAxis/Debug/UI_DebugView.PointStart` Point _ui_debug))
    (:`else`)))

(event `/CoordinateAxis/Debug/BPI_DrawInfo.BPI_SendEnd2`
  (params (Point :type "Vector2D Structure"))
  (bind _ui_debug (`self.UI_Debug`)
    (:`then`
      (set `/CoordinateAxis/Debug/UI_DebugView.PointEnd` Point _ui_debug))
    (:`else`)))

(event `/CoordinateAxis/Debug/BPI_DrawInfo.BPI_SendStart1`
  (params (Point :type "Vector2D Structure"))
  (bind _ui_debug (`self.UI_Debug`)
    (:`then`
      (set `/CoordinateAxis/Debug/UI_DebugView.MoveStart` Point _ui_debug))
    (:`else`)))

(event `/CoordinateAxis/Debug/BPI_DrawInfo.BPI_SendEnd1`
  (params (Point :type "Vector2D Structure"))
  (bind _ui_debug (`self.UI_Debug`)
    (:`then`
      (set `/CoordinateAxis/Debug/UI_DebugView.MoveEnd` Point _ui_debug))
    (:`else`)))

(event `/CoordinateAxis/Debug/BPI_DrawInfo.BPI_SendAngle`
  (params (Angle :type "Float (single-precision)"))
  (bind _ui_debug (`self.UI_Debug`)
    (:`then`
      (set `/CoordinateAxis/Debug/UI_DebugView.Angle` Angle _ui_debug))
    (:`else`)))

(fn `UserConstructionScript`)